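; Floor actor that can be highlighted on selection and right-clicked to open a menu for editing its texture.
; Selected and NoSelected, bound to Depth and NoDepth events at BeginPlay, toggle the mesh's custom depth for an outline and set IsSelected.
; RightClick_Floor acts only when the caller is itself, alternating between opening MaterialFloor after clearing roof, wall and floor material widgets, and removing MaterialFloor.
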(event `self.ReceiveBeginPlay`
  ;[1 1 1] Outline
  (add `self.Depth` (delegate `Selected`))
  (add `self.NoDepth` (delegate `NoSelected`)))

(event `RightClick_Floor`
  (params (caller :type "Actor Object Reference"))
  ;[1 1 1] Edit Floor Texture
  (if (== caller self)
    (`/Engine/EditorBlueprintResources/StandardMacros.FlipFlop`
      (:`A`
        (bind _foundwidgets (`WidgetBlueprintLibrary.GetAllWidgetsOfClass` "/Game/UI/MaterialRoof.MaterialRoof_C"))
        (for _array_element _foundwidgets
          (`Widget.RemoveFromParent` _array_element))
        (bind _foundwidgets_2 (`WidgetBlueprintLibrary.GetAllWidgetsOfClass` "/Game/UI/MaterialWalls.MaterialWalls_C"))
        (for _array_element_2 _foundwidgets_2
          (`Widget.RemoveFromParent` _array_element_2))
        (bind _foundwidgets_3 (`WidgetBlueprintLibrary.GetAllWidgetsOfClass` "/Game/UI/MaterialFloor.MaterialFloor_C"))
        (for _array_element_3 _foundwidgets_3
          (`Widget.RemoveFromParent` _array_element_3))
        (bind _returnvalue (`|CreateWidget` "/Game/UI/MaterialFloor.MaterialFloor_C" (`GameplayStatics.GetPlayerController` 0)))
        (`UserWidget.AddToViewport` _returnvalue 0))
      (:`B`
        (bind _foundwidgets_4 (`WidgetBlueprintLibrary.GetAllWidgetsOfClass` "/Game/UI/MaterialFloor.MaterialFloor_C"))
        (for _array_element_4 _foundwidgets_4
          (`Widget.RemoveFromParent` _array_element_4))))))

(event `Selected`
  ;[1 1 1] Outline
  (`PrimitiveComponent.SetRenderCustomDepth` (`self.StaticMesh`) true)
  (set `self.IsSelected` true))

(event `NoSelected`
  ;[1 1 1] Outline
  (`PrimitiveComponent.SetRenderCustomDepth` (`self.StaticMesh`) false)
  (set `self.IsSelected` false))

(fn `UserConstructionScript`)