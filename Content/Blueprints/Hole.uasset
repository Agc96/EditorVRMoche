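; Hole actor that drops an editor character that hits it and later returns it to the start.
; On hit, it teleports the character to a height just below world zero at the same XY, then after a delay moves it to the first PlayerStart found.
; Bound selection events toggle Custom Depth on its sphere for an outline.
; An unconnected loop for destroying other actors never runs.
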(event `CustomEvent`
  ;[1 1 1] Outline
  (add `self.Depth` (delegate `Selected`))
  (add `self.NoDepth` (delegate `NoSelected`)))

(event `Selected`
  ;[1 1 1] Outline
  (`PrimitiveComponent.SetRenderCustomDepth` (`self.Sphere`) true))

(event `NoSelected`
  ;[1 1 1] Outline
  (`PrimitiveComponent.SetRenderCustomDepth` (`self.Sphere`) false))

(event `self.ReceiveHit`
  (params (MyComp :type "PrimitiveComponent Object Reference") (Other :type "Actor Object Reference") (OtherComp :type "PrimitiveComponent Object Reference") (bSelfMoved :type Boolean) (HitLocation :type "Vector Structure") (HitNormal :type "Vector Structure") (NormalImpulse :type "Vector Structure") (Hit :type "HitResult Structure (by ref)"))
  ;[1 1 1] Caída
  (bind _aseditor_character (cast `/Game/Blueprints/EditorCharacter` Other))
  (bind _rootcomponent (`Actor.RootComponent` _aseditor_character))
  (`SceneComponent.K2_SetWorldLocation` _rootcomponent (+ (* (`self.K2_GetActorLocation` _aseditor_character) (1.0 1.0 0.0)) (0.0 0.0 -20.0)) false false)
  (bind _outactors (`GameplayStatics.GetAllActorsOfClass` "/Game/Blueprints/PlayerStart.PlayerStart_C"))
  (`KismetSystemLibrary.Delay` 10.0)
  (`SceneComponent.K2_SetWorldLocation` _rootcomponent (`self.K2_GetActorLocation` (`|GetArrayItem` _outactors)) false false))

(fn `UserConstructionScript`)