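; EditableObject is a clickable actor for an in-game editor that either opens an options widget or deletes itself, depending on the game instance's EditorMode.
; Every click also calls NoDepth on all EditableObjects, then Depth on itself, apparently to highlight the selection.
; Right mouse sends the actor under the cursor to TextureF on Wall, Floor and Roof references, whose casts never execute.
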(event MouseInput|EventActorOnClicked
  (params (ButtonPressed :type Key%20Structure))
  (Utilities|FlowControl|Sequence
    (:then_0
      (bind _aseditor_game_instance (Utilities|Casting|CastToEditorGameInstance (Game|GetGameInstance)))
      (switch Utilities|FlowControl|Switch|SwitchonEditorMode (Variables|/Game/Blueprints/EditorGameInstance.EditorGameInstance_C|GetEditorMode _aseditor_game_instance)
        (:NewEnumerator0
          ;[1 1 1] Abrir ventana de opciones del objeto
          (bind _foundwidgets (Widget|GetAllWidgetsOfClass "/Game/UI/Options.Options_C" true))
          (for _array_element _foundwidgets
            (Widget|RemovefromParent _array_element))
          (bind _returnvalue (UserInterface|CreateWidget "/Game/UI/EditableObjectOptions.EditableObjectOptions_C" (Game|GetPlayerController 0) self))
          (UserInterface|Viewport|AddtoViewport _returnvalue 0))
        (:NewEnumerator2
          ;[1 1 1] Eliminar objeto
          (bind _foundwidgets_2 (Widget|GetAllWidgetsOfClass "/Game/UI/EditableObjectOptions.EditableObjectOptions_C" true))
          (for _array_element_2 _foundwidgets_2
            (bind _aseditable_object_options (Utilities|Casting|CastToEditableObjectOptions _array_element_2))
            (if (== (Variables|/Game/UI/EditableObjectOptions.EditableObjectOptions_C|GetSelectedObject _aseditable_object_options) self)
              (Widget|RemovefromParent _aseditable_object_options)))
          (Actor|DestroyActor))))
    (:then_1
      (bind _outactors (Actor|GetAllActorsOfClass "EditableObject_C"))
      (for _array_element_3 _outactors
        (Default|CallNoDepth _array_element_3)))
    (:then_2
      (Default|CallDepth))))

(event EventBeginPlay
  (Input|EnableInput (Game|GetPlayerController 0)))

(event Input|MouseEvents|RightMouseButton
  (params (Key :type Key%20Structure))
  (:Pressed
    (Default|CallTextureF (stale _aswall) (.HitActor (Collision|BreakHitResult (.HitResult (Game|Player|GetHitResultUnderCursorbyChannel (Game|GetPlayerController 0) "TraceTypeQuery1" true)))))))

(fn ConstructionScript)