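; PlayerLocation is a clickable player start marker for an in-game editor that opens its options window when clicked.
; On click it reads the editor mode from EditorGameInstance and responds in Normal mode.
; It removes any open top-level EditableOptions widgets, then creates a PlayerLocationOptions widget bound to itself and adds it to the viewport.
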(event `self.ReceiveActorOnClicked`
  (params (ButtonPressed :type "Key Structure"))
  (bind _aseditor_game_instance (cast `/Game/Blueprints/EditorGameInstance` (`GameplayStatics.GetGameInstance`)))
  (switch `/Game/Blueprints/EditorMode` (`/Game/Blueprints/EditorGameInstance.EditorMode` _aseditor_game_instance)
    (:`NewEnumerator0`
      ;[1 1 1] Abrir ventana de opciones del objeto
      (bind _foundwidgets (`WidgetBlueprintLibrary.GetAllWidgetsOfClass` "/Game/UI/EditableOptions.EditableOptions_C"))
      (for _array_element _foundwidgets
        (`Widget.RemoveFromParent` _array_element))
      (bind _returnvalue (`|CreateWidget` "/Game/UI/PlayerLocationOptions.PlayerLocationOptions_C" (`GameplayStatics.GetPlayerController` 0) self))
      (`UserWidget.AddToViewport` _returnvalue 0))))

(fn `UserConstructionScript`)