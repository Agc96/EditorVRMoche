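; EditableDoorButton is a selectable door button actor linked to EditableDoor actors by a wall ID.
; On BeginPlay it binds selection events that toggle custom depth on the button mesh for an outline and track IsSelected, then stores its object name as text.
; When destroyed, it searches all EditableDoor actors and destroys any whose DoorWallID matches its ButtonWallID.
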(event `self.ReceiveBeginPlay`
  ;[1 1 1] Outline
  (add `self.Depth` (delegate `Selected`))
  (add `self.NoDepth` (delegate `NoSelected`))
  (set `self.ObjectName_` (`KismetTextLibrary.Conv_StringToText` (`KismetSystemLibrary.GetObjectName` self))))

(event `NoSelected`
  ;[1 1 1] Outline
  (`PrimitiveComponent.SetRenderCustomDepth` (`self.DoorButton`) false)
  (set `self.IsSelected` false))

(event `Selected`
  ;[1 1 1] Outline
  (`PrimitiveComponent.SetRenderCustomDepth` (`self.DoorButton`) true)
  (set `self.IsSelected` true))

(event `self.ReceiveDestroyed`
  (bind _outactors (`GameplayStatics.GetAllActorsOfClass` "/Game/Blueprints/EditableDoor.EditableDoor_C"))
  (for _array_element _outactors
    (if (`KismetTextLibrary.EqualEqual_TextText` (`/Game/Blueprints/EditableDoor.DoorWallID` _array_element) (`self.ButtonWallID`))
      (`self.K2_DestroyActor` _array_element))))

(fn `UserConstructionScript`)