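; EditorCharacter is a player-controlled character with a spring-arm camera, driven by input events for movement, look and zoom.
; Forward and right movement follow the control yaw only, while MoveUp uses actor location plus a scaled up vector as its direction.
; Turn and look inputs are scaled by rate variables and delta time.
; Zoom steps the spring arm length, with a minimum check on zoom-in and no limit on zoom-out.
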(event `InputAxis|MoveForward`
  (params (AxisValue :type "Float (single-precision)"))
  ;[1 1 1] Movimientos
  (`self.AddMovementInput` (`KismetMathLibrary.GetForwardVector` (`KismetMathLibrary.MakeRotator` 0.0 0.0 (.yaw (`self.GetControlRotation`)))) AxisValue))

(event `InputAxis|MoveUp`
  (params (AxisValue :type "Float (single-precision)"))
  ;[1 1 1] Move up/down
  (`self.AddMovementInput` (+ (`self.K2_GetActorLocation` self) (* (`self.GetActorUpVector` self) (`self.Constante`))) AxisValue))

(event `InputAction|ZoomIn`
  (params (Key :type "Key Structure"))
  (bind _springarm (`self.SpringArm`))
  (bind _targetarmlength (`SpringArmComponent.TargetArmLength` _springarm))
  ;[1 1 1] ZoomIn
  (:`Pressed`
    (set `self.CameraDistance` _targetarmlength)
    (if (>= (`self.CameraDistance`) (`self.MinCameraDistance`))
      (set `SpringArmComponent.TargetArmLength` (- _targetarmlength 50.0) _springarm))))

(event `InputAxis|MoveRight`
  (params (AxisValue :type "Float (single-precision)"))
  ;[1 1 1] Movimientos
  (`self.AddMovementInput` (`KismetMathLibrary.GetRightVector` (`KismetMathLibrary.MakeRotator` 0.0 0.0 (.yaw (`self.GetControlRotation`)))) AxisValue))

(event `InputAxis|LookUp`
  (params (AxisValue :type "Float (single-precision)"))
  ;[1 1 1] Cameraturn up/down
  (`self.AddControllerPitchInput` (* AxisValue (`self.CameraLookRate`) (`GameplayStatics.GetWorldDeltaSeconds`))))

(event `InputAxis|Turn`
  (params (AxisValue :type "Float (single-precision)"))
  ;[1 1 1] Camera turn rigth/left
  (`self.AddControllerYawInput` (* AxisValue (`self.CameraTurnRate`) (`GameplayStatics.GetWorldDeltaSeconds`))))

(event `InputAction|ZoomOut`
  (params (Key :type "Key Structure"))
  (bind _springarm (`self.SpringArm`))
  (bind _targetarmlength (`SpringArmComponent.TargetArmLength` _springarm))
  ;[1 1 1] ZoomOut
  (:`Pressed`
    (set `self.CameraDistance` _targetarmlength)
    (set `SpringArmComponent.TargetArmLength` (+ _targetarmlength 50.0) _springarm)))

(fn `UserConstructionScript`)